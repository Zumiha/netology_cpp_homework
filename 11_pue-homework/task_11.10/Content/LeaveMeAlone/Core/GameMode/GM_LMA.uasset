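; Game mode for LeaveMeAlone that runs the level countdown and handles both ways a match ends.
; On BeginPlay it starts a looping one-second GameTime timer and binds to OnDeath on the player character's HealthComponent.
; At zero it clears the timer, fires TimerExpire, pauses and shows W_GameEnd; death shows W_GameOver after a short delay without pausing.
; Both screens switch to UI-only input with a visible cursor.
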(event Custom|LevelTimer_Expire
  (bind _returnvalue (Game|GetPlayerController 0))
  (bind _output_get (Variables|Default|SetGameTime (- (Variables|Default|GetGameTime) 1)))
  (if (== _output_get 0)
    (Utilities|Time|ClearandInvalidateTimerbyHandle (Variables|Default|GetGameTimerHandle))
    (Default|CallTimerExpire "Hidden")
    (Game|SetGamePaused true)
    (bind _returnvalue_2 (UserInterface|CreateWidget "/Game/LeaveMeAlone/UI/W_GameEnd.W_GameEnd_C"))
    (UserInterface|Viewport|AddtoViewport _returnvalue_2 0)
    (Widget|SetVisibility _returnvalue_2 "Visible")
    (Input|SetInputModeUIOnly _returnvalue _returnvalue_2 "DoNotLock" true)
    (Variables|/Script/Engine.PlayerController|SetbShowMouseCursor _returnvalue true)))

(event Custom|PlayerDeath
  (Utilities|Time|SetTimerbyEvent (delegate Custom|PlayerAfterLife) 1.0))

(event Custom|PlayerAfterLife
  (bind _returnvalue (Game|GetPlayerController 0))
  (bind _returnvalue_2 (UserInterface|CreateWidget "/Game/LeaveMeAlone/UI/W_GameOver.W_GameOver_C"))
  (UserInterface|Viewport|AddtoViewport _returnvalue_2 0)
  (Widget|SetVisibility _returnvalue_2 "Visible")
  (Input|SetInputModeUIOnly _returnvalue _returnvalue_2 "DoNotLock" true)
  (Variables|/Script/Engine.PlayerController|SetbShowMouseCursor _returnvalue true))

(event EventBeginPlay
  (bind _returnvalue (Utilities|Time|SetTimerbyEvent (delegate Custom|LevelTimer_Expire) 1.0 true))
  (Variables|Default|SetGameTimerHandle _returnvalue)
  (bind _healthcomponent (CallFunction|NewFunction))
  (EventDispatchers|BindEventtoOnDeath _healthcomponent (delegate Custom|PlayerDeath)))

(event EventTick
  (params (DeltaSeconds :type Float%20%28single-precision%29)))

(fn ConstructionScript)

(fn GetPlayerCasttoLMADeafultCharacter
  (bind _aslmadefault_character (Utilities|Casting|CastToLMADefaultCharacter (Game|Player|GetPlayerPawn 0))
    (:then
      _)
    (:CastFailed
      _))
  (return _aslmadefault_character))

(fn NewFunction
  (bind _aslmadefault_character (Utilities|Casting|CastToLMADefaultCharacter (Game|Player|GetPlayerPawn 0))
    (:then
      _)
    (:CastFailed
      _))
  (return (Variables|/Script/LeaveMeAlone.LMADefaultCharacter|GetHealthComponent _aslmadefault_character)))